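; Player pawn for an on-rails shooter that travels along the BP_SplineTool spline with a visible mouse cursor.
; Tick advances spline distance to place the root, while axis inputs offset SpringArm1 for on-screen movement.
; Held fire loops through a gate and retriggerable delay, line-tracing toward the cursor; hit results are unused.
; Right-click triggers a timed double-attack-speed power-up or an empty LASER stub.
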(event Custom|Activate%20DAS
  ;[1 1 1] Activates Double Attack Speed (DAS)
  (Variables|Default|SetShot%20Delay (/ (Variables|Default|GetShot%20Delay) 2.0))
  (bind _newtrack_0 (Timeline|Duration%20of%20DAS Play)
    (:Update
      (Variables|Default|SetDurationofDAS _newtrack_0)
      (Utilities|FlowControl|Delay 1e+01)
      (Variables|Default|SetShot%20Delay (* (Variables|Default|GetShot%20Delay) 2.0))
      (Variables|Default|SethasDAS false))))

(event Custom|Activate%20LASER)

(event EventBeginPlay
  ;[1 0.9488 0.2575] Get reference to BP_SplineTool
  (bind _returnvalue (Actor|GetActorOfClass "/Game/Blueprints/BP_SplineTool.BP_SplineTool_C"))
  (Variables|Default|SetSplineRef _returnvalue)
  (Variables|/Script/Engine.PlayerController|SetbShowMouseCursor (Game|GetPlayerController 0) true))

(event EventTick
  (params (DeltaSeconds :type Float%20%28single-precision%29))
  (bind _splineref (Variables|Default|GetSplineRef))
  (bind _playership (Variables|Default|GetPlayerShip))
  (bind _spline (Variables|/Game/Blueprints/BP_SplineTool.BP_SplineTool_C|GetSpline _splineref))
  ;[0.6723 1 0.3645] Move along spline
  (bind _output_get (Variables|Default|Setdistance (+ (* (* DeltaSeconds 25.0) (Variables|Default|GetSplineSpeed)) (Variables|Default|Getdistance))))
  (Transformation|SetWorldLocationAndRotation (Variables|Default|GetRoot) (Spline|GetLocationatDistanceAlongSpline _spline _output_get "World") (Math|Rotator|MakeRotator 0.0 (.pitch (Spline|GetRotationatDistanceAlongSpline _spline _output_get "World")) (.yaw (Spline|GetRotationatDistanceAlongSpline _spline _output_get "World"))) true false)
  (Transformation|SetWorldRotation _playership (Math|Rotator|FindLookatRotation (Transformation|GetWorldLocation _playership) (Transformation|GetWorldLocation (Variables|Default|GetSpringArm1))) false false))

(event Input|ActionEvents|InputActionFire
  (params (Key :type Key%20Structure :default "None"))
  (bind _returnvalue (Game|GetPlayerController 0))
  (bind (_worldlocation _worlddirection) (Game|Player|ConvertMouseLocationToWorldSpace _returnvalue))
  ;[1 1 1] Shoot Gun
  (:Pressed
    (Utilities|FlowControl|Sequence
      (:then_0
        (goto _label Open))
      (:then_1
        (Utilities|FlowControl|Gate true :!label _label
          (:Exit
            (Utilities|FlowControl|Sequence
              (:then_0
                (Audio|PlaySound2D "/Game/Sound/GunShot/GunShotCue.GunShotCue" 1.0 1.0 0.0 0 0)
                (bind _outhit (Collision|LineTraceByChannel (Transformation|GetWorldLocation (Variables|Default|GetShootLoc)) (+ _worldlocation (* _worlddirection (+ (Variables|Default|GetWeaponRange) 5e+03))) "TraceTypeQuery1" false 0 "Persistent")))
              (:then_1
                (Utilities|FlowControl|RetriggerableDelay (Variables|Default|GetShot%20Delay))
                (goto _label))))))))
  (:Released
    (goto _label Close)))

(event Input|AxisEvents|InputAxisMoveForward
  (params (AxisValue :type Float%20%28single-precision%29))
  (bind _returnvalue (Math|Vector|MakeVector 0.0 0.0 AxisValue))
  (bind _movementspeed (Variables|Default|GetMovementSpeed))
  (bind _returnvalue_2 (Math|Vector|ClampVectorSize _returnvalue 0.0 1.0))
  (bind _returnvalue_3 (* AxisValue _movementspeed))
  (bind _returnvalue_4 (* _returnvalue_2 _returnvalue_3))
  ;[0.3278 0.6654 1] Up Movement On Screen
  (if (> (Math|Vector|VectorLength _returnvalue_4) 0.0)
    (Transformation|AddLocalOffset (Variables|Default|GetSpringArm1) _returnvalue_4 true false)))

(event Input|AxisEvents|InputAxisMoveRight
  (params (AxisValue :type Float%20%28single-precision%29))
  (bind _returnvalue (Math|Vector|MakeVector 0.0 AxisValue 0.0))
  (bind _movementspeed (Variables|Default|GetMovementSpeed))
  (bind _returnvalue_2 (Math|Vector|ClampVectorSize _returnvalue 0.0 1.0))
  (bind _returnvalue_3 (* AxisValue _movementspeed))
  (bind _returnvalue_4 (* _returnvalue_2 _returnvalue_3))
  ;[0.3278 0.6654 1] Right Movement On Screen
  (if (> (Math|Vector|VectorLength _returnvalue_4) 0.0)
    (Transformation|AddLocalOffset (Variables|Default|GetSpringArm1) _returnvalue_4 true false)))

(event Input|AxisEvents|InputAxisMoveBack
  (params (AxisValue :type Float%20%28single-precision%29))
  (bind _returnvalue (Math|Vector|MakeVector 0.0 0.0 AxisValue))
  (bind _movementspeed (Variables|Default|GetMovementSpeed))
  (bind _returnvalue_2 (Math|Vector|ClampVectorSize _returnvalue 0.0 -1.0))
  (bind _returnvalue_3 (* AxisValue _movementspeed))
  (bind _returnvalue_4 (* _returnvalue_2 _returnvalue_3))
  ;[0.3278 0.6654 1] Down Movement On Screen
  (if (> (Math|Vector|VectorLength _returnvalue_4) 0.0)
    (Transformation|AddLocalOffset (Variables|Default|GetSpringArm1) _returnvalue_4 true false)))

(event Input|AxisEvents|InputAxisMoveLeft
  (params (AxisValue :type Float%20%28single-precision%29))
  (bind _returnvalue (Math|Vector|MakeVector 0.0 AxisValue 0.0))
  (bind _movementspeed (Variables|Default|GetMovementSpeed))
  (bind _returnvalue_2 (Math|Vector|ClampVectorSize _returnvalue 0.0 -1.0))
  (bind _returnvalue_3 (* AxisValue _movementspeed))
  (bind _returnvalue_4 (* _returnvalue_2 _returnvalue_3))
  ;[0.3278 0.6654 1] Left Movement On Screen
  (if (> (Math|Vector|VectorLength _returnvalue_4) 0.0)
    (Transformation|AddLocalOffset (Variables|Default|GetSpringArm1) _returnvalue_4 true false)))

(event Input|MouseEvents|RightMouseButton
  (params (Key :type Key%20Structure :default "None"))
  ;[1 1 1] Use PowerUps
  (:Pressed
    (if (Variables|Default|GethasDAS)
      (CallFunction|ActivateDAS)
      (elif (Variables|Default|GethasLASER)
        (CallFunction|ActivateLASER)))))

(fn ConstructionScript)